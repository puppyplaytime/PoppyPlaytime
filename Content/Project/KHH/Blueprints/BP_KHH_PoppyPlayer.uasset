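; Player Blueprint that freezes a sensed KHH_Enemy while that enemy's AI controller has line of sight to the player.
; The Sensor stores seen enemies not tagged "Del", and Tick toggles the stored enemy's CustomTimeDilation between stopped and normal.
; Tick also calls Play on the JumpScare component whenever it renders in the main pass.
; Overlapping a KHH_Enemy stores it as Teacher, which this graph never reads.
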(event OnSeePawn(sensor)
  (params (Pawn :type Pawn%20Object%20Reference))
  (bind _askhh_enemy (Utilities|Casting|CastToKHH_Enemy Pawn))
  (if (not (Actor|ActorHasTag _askhh_enemy "Del"))
    (Variables|Default|SetEnemy _askhh_enemy)))

(event EventBeginPlay)

(event Collision|EventActorBeginOverlap
  (params (OtherActor :type Actor%20Object%20Reference))
  (bind _askhh_enemy (Utilities|Casting|CastToKHH_Enemy OtherActor))
  (Variables|Default|SetTeacher _askhh_enemy))

(event EventTick
  (params (DeltaSeconds :type Float%20%28single-precision%29))
  (bind _enemy (Variables|Default|GetEnemy))
  (bind _enemy_2 (Variables|Default|GetEnemy))
  (bind _enemy_3 (Variables|Default|GetEnemy))
  (Utilities|FlowControl|Sequence
    (:then_0
      (Utilities|IsValid _enemy_3
        (:Is%20Valid
          (if true
            (bind _asaicontroller (Utilities|Casting|CastToAIController (Pawn|GetController _enemy_3)))
            (if (Controller|LineOfSightTo _asaicontroller (Game|GetPlayerCharacter 0) "0, 0, 0" false)
              (Variables|/Script/Engine.Actor|SetCustomTimeDilation _enemy_2 0.0)
              (Variables|/Script/Engine.Pawn|SetbUseControllerRotationYaw _enemy_2 true)
              (else
                (Variables|/Script/Engine.Actor|SetCustomTimeDilation _enemy 1.0)
                (Variables|/Script/Engine.Pawn|SetbUseControllerRotationYaw _enemy true)))))))
    (:then_1
      (if (Variables|/Script/Engine.PrimitiveComponent|GetbRenderInMainPass (Variables|Default|GetJumpScare))
        (Audio|Components|Audio|Play (Variables|Default|GetJumpScare) false)))))

(fn ConstructionScript)