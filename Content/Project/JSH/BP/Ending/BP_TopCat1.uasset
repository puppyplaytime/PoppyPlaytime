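; Ending-sequence actor that stages the NappyCat death scene and finale.
; Once EndingVisible is set, Tick waits briefly, reveals the skeletal mesh, loops its death animation and arms the overlap via NION.
; An armed overlap hides the player's hands and arms, plays the death sound, replaces the UI with a movie widget and shows hand VFX.
; Chained delays then reveal fire, add ending widgets, flag BP_Random's sound off and start ending music.
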(event EventBeginPlay)

(event Collision|EventActorBeginOverlap
  (params (OtherActor :type Actor%20Object%20Reference))
  (if (Variables|Default|GetNION)
    (Utilities|FlowControl|Sequence
      (:then_0
        (bind _asbp_poppy_player (Utilities|Casting|CastToBP_PoppyPlayer (Game|Player|GetPlayerPawn 0)))
        (bind _output_get (Variables|/Script/CatTeacher.KMK_Player|SetHands _asbp_poppy_player (Variables|/Script/CatTeacher.KMK_Player|GetHands _asbp_poppy_player)))
        (for (_array_element _array_index) _output_get
          (Utilities|FlowControl|Sequence
            (:then_0
              (switch int _array_index
                (:Default
                  _)
                (:0
                  _)
                (:1
                  _))
              (bind _output_get_2 (Variables|/Script/CatTeacher.KMK_PlayerHand|Sethand _array_element (Variables|/Script/CatTeacher.KMK_PlayerHand|Gethand _array_element)))
              (Class|PrimitiveComponent|SetRenderinMainPass _output_get_2 false)
              (Class|PrimitiveComponent|SetRenderinDepthPass _output_get_2 false))
            (:then_1
              (Class|PrimitiveComponent|SetRenderinMainPass (Variables|/Script/CatTeacher.KMK_Player|GetarmMesh _asbp_poppy_player) false)
              (Class|PrimitiveComponent|SetRenderinDepthPass (Variables|/Script/CatTeacher.KMK_Player|GetarmMesh _asbp_poppy_player) false)))))
      (:then_1
        (Rendering|SetVisibility (Variables|Default|GetN_HandVFX1) true false)
        (Utilities|FlowControl|Delay 4.5)
        (Utilities|FlowControl|Sequence
          (:then_0
            (Rendering|SetVisibility (Variables|Default|Getfire) true false)
            (Utilities|FlowControl|Delay 5.0)
            (bind _returnvalue (UserInterface|CreateWidget "/Game/Project/UI/WBP_Ending.WBP_Ending_C"))
            (UserInterface|Viewport|AddtoViewport _returnvalue 3)
            (Utilities|FlowControl|Delay 7.0)
            (bind _outactors (Actor|GetAllActorsOfClass "/Game/Project/JSH/BP/BP_Random.BP_Random_C"))
            (bind _output_get_3 (Variables|Default|SetRandom _outactors))
            ;[1 1 1] Cast 해와서 사운드 꺼줘야함
            (bind _asbp_random (Utilities|Casting|CastToBP_Random (Utilities|Array|Get(acopy) _output_get_3)))
            (Variables|/Script/CatTeacher.JSH_Random|SetEndingSoundOff _asbp_random true)
            (Audio|PlaySound2D "/Game/Project/JSH/Audio/onwards-and-downwards.onwards-and-downwards" 1.0 1.0 0.0 0 0)
            (bind _returnvalue_2 (UserInterface|CreateWidget "/Game/Project/JSH/BP/Ending/WBP_Ending_KHH2.WBP_Ending_KHH2_C"))
            (UserInterface|Viewport|AddtoViewport _returnvalue_2 3))))
      (:then_2
        (Audio|PlaySoundatLocation "/Game/Project/JSH/Audio/catnap-boss_die.catnap-boss_die" (Transformation|GetActorLocation) "0, 0, 0" 1.0 1.0 0.0 0 0 0 0))
      (:then_3
        (Viewport|RemoveAllWidgets)
        (bind _returnvalue_3 (UserInterface|CreateWidget "/Game/Project/JSH/BP/Ending/BP_EMoive.BP_EMoive_C"))
        (UserInterface|Viewport|AddtoViewport _returnvalue_3 3)))))

(event EventTick
  (params (DeltaSeconds :type Float%20%28single-precision%29))
  (if (Variables|Default|GetEndingVisible)
    (Utilities|FlowControl|Delay 2.0)
    (Rendering|SetVisibility (Variables|Default|GetSkeletalMesh) true false)
    (Utilities|FlowControl|Sequence
      (:then_0
        (if (not (Variables|Default|GetisAnim))
          (Components|Animation|PlayAnimation (Variables|Default|GetSkeletalMesh) "/Game/Project/JSH/Asset/4/source/Armature_A_NappyCat_NappyCatDeath.Armature_A_NappyCat_NappyCatDeath" true)
          (Variables|Default|SetisAnim true)))
      (:then_1
        (Variables|Default|SetNION true)))))

(fn ConstructionScript)